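; MyDummy is an actor that shows a skeletal pose loaded from a saved text file.
; On BeginPlay it loads the Idle pose from a hardcoded absolute path into a poseable mesh, then hides the skeletal mesh and shows the posed one.
; A RecordBones event saves the skeletal mesh's current bone positions to an Idle text file under SaveDirectory, which InitSkeleton can load back.
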(event `self.ReceiveBeginPlay`
  (bind _poseablemesh (`self.PoseableMesh`))
  (`self.InitSkeleton` "C:\\Users\\comma\\Desktop\\Repos\\AnimFinal\\Content\\SavedPositions\\Idle.txt")
  (`SceneComponent.SetVisibility` (`self.Mesh`) false false)
  (`SceneComponent.SetVisibility` _poseablemesh true false)
  (`SceneComponent.K2_SetRelativeRotation` _poseablemesh (struct) false false))

(event `self.ReceiveTick`
  (params (DeltaSeconds :type "Float (single-precision)")))

(event `RecordBones`
  (`self.RecordPosition` (`self.Mesh`) (`KismetStringLibrary.Concat_StrStr` (`KismetStringLibrary.Concat_StrStr` (`self.Save Directory`) "Idle") ".txt")))

(event `InitSkeleton`
  (params (File :type String))
  (`self.LoadSkeletonPosition` (`self.PoseableMesh`) File))

(fn `UserConstructionScript`)